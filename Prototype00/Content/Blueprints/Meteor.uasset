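; Meteor actor Blueprint with a Sphere component, pinned to world height zero every frame.
; Tick sets both the actor and the Sphere to their current X and Y, with Z computed as Z minus itself, so neither descends gradually.
; The moves are unswept, and the Sphere call also passes a default rotation.
; BeginPlay, overlap and the construction script have no logic.
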(event EventBeginPlay)

(event Collision|EventActorBeginOverlap
  (params (OtherActor :type Actor%20Object%20Reference)))

(event EventTick
  (params (DeltaSeconds :type Float%20%28single-precision%29))
  (bind _returnvalue (Transformation|GetActorLocation))
  (bind _sphere (Variables|Default|GetSphere))
  (bind (_x _y _z) (Math|Vector|BreakVector _returnvalue))
  (bind _returnvalue_2 (Transformation|GetWorldLocation _sphere))
  (bind (_x_2 _y_2 _z_2) (Math|Vector|BreakVector _returnvalue_2))
  (Transformation|SetActorLocation (Math|Vector|MakeVector _x _y (- _z _z)) false false)
  (Transformation|SetWorldLocationAndRotation _sphere (Math|Vector|MakeVector _x_2 _y_2 (- _z_2 _z_2)) "0, 0, 0" false false))

(fn ConstructionScript)