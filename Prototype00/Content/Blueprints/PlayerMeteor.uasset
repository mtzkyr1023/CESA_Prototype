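; PlayerMeteor is a player-controlled physics sphere that is pushed in the direction the camera faces.
; Pressing Z makes Tick apply one horizontal impulse along the camera's forward vector, then clear the flag.
; Holding Left or Right steps a yaw angle every frame (not delta-scaled) to rotate the spring arm, steering the push.
; The angle is debug-printed, and a RunningTime cooldown check is left unconnected.
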(event EventBeginPlay
  (|CallParentFunction)
  (Input|EnableInput (Game|GetPlayerController 0)))

(event Collision|EventActorBeginOverlap
  (params (OtherActor :type Actor%20Object%20Reference))
  (|CallParentFunction OtherActor) ; This node is disabled and will not be called.\nDrag off pins to build functionality.
)

(event EventTick
  (params (DeltaSeconds :type Float%20%28single-precision%29))
  (bind _impulse (Variables|Default|GetImpulse))
  (bind _camera (Variables|Default|GetCamera))
  (bind _rotatehori (Variables|Default|GetRotateHori))
  (bind _returnvalue (Math|Vector|GetForwardVector _camera))
  (bind _returnvalue_2 (Math|Vector|Normalize _returnvalue))
  (bind (_x _y) (Math|Vector|BreakVector _returnvalue_2))
  (|CallParentFunction DeltaSeconds)
  (if (Variables|Default|GetCanPush)
    (Physics|AddImpulse (Variables|Default|GetSphere) (Math|Vector|MakeVector (* _x _impulse) (* _y _impulse) 0.0) "None" false)
    (Variables|Default|SetCanPush false)
    (else
      (bind _output_get (Variables|Default|SetRunningTime (+ (Variables|Default|GetRunningTime) 1.0)))))
  (if (Variables|Default|GetLeftRot)
    (Math|Float|DecrementFloat _rotatehori
      (:%20%20
        _)))
  (if (Variables|Default|GetRightRot)
    (Math|Float|IncrementFloat _rotatehori
      (:%20%20
        _)))
  (Transformation|SetWorldRotation (Variables|Default|GetSpringArm) (Math|Vector|RotatorfromAxisandAngle "0, 0,1.000000" _rotatehori) false false)
  (Development|PrintString (Utilities|String|ToString(Float) _rotatehori) true true "(R=0.000000,G=0.660000,B=1.000000,A=1.000000)" 0.0))

(event Input|KeyboardEvents|Z
  (params (Key :type Key%20Structure))
  (:Pressed
    (Variables|Default|SetCanPush true))
  (:Released
    (Variables|Default|SetCanPush false)))

(event Input|KeyboardEvents|Left
  (params (Key :type Key%20Structure))
  (:Pressed
    (Variables|Default|SetLeftRot true))
  (:Released
    (Variables|Default|SetLeftRot false)))

(event Input|KeyboardEvents|Right
  (params (Key :type Key%20Structure))
  (:Pressed
    (Variables|Default|SetRightRot true))
  (:Released
    (Variables|Default|SetRightRot false)))

(fn ConstructionScript
  (|CallParentFunction))